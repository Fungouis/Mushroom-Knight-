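; Paper2D treasure chest that opens once when the player character overlaps it and releases a pickup.
; An overlap on the Closed component adds a non-looping Chest flipbook component at runtime to play the animation.
; After a short delay it spawns BP_pickup at the chest's transform and destroys RenderComponent and Closed, leaving the flipbook in place.
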(event OnComponentBeginOverlap(closed)
  (params (OverlappedComponent :type Primitive%20Component%20Object%20Reference) (OtherActor :type Actor%20Object%20Reference) (OtherComp :type Primitive%20Component%20Object%20Reference) (OtherBodyIndex :type Integer) (bFromSweep :type Boolean) (SweepResult :type Hit%20Result%20Structure%20%28by%20ref%29))
  ;[0.15 0.15 0.15 0.5] overlaps to player
  (Utilities|Casting|CastToBP_Charchter OtherActor)
  ;[0.15 0.15 0.15 0.5] does it onces
  (Utilities|FlowControl|DoOnce false
    (:Completed
      ;[0.15 0.15 0.15 0.5] adds flip book
      (bind _returnvalue (AddComponent|AddPaperFlipbookComponent false))
      ;[0.15 0.15 0.15 0.5] adds chest flip book set looping to faluse
      (Sprite|SetFlipbook _returnvalue "/Game/Tilemaps/Sprites/chest.chest")
      (Components|Timeline|SetLooping _returnvalue false)
      ;[0.15 0.15 0.15 0.5] delay
      (Utilities|FlowControl|Delay 0.2)
      ;[0.15 0.15 0.15 0.5] spawns  pick up
      (Game|SpawnActorfromClass "/Game/Pickups/BP_pickup.BP_pickup_C" (Transformation|GetActorTransform) "Undefined" "MultiplyWithRoot" 0 0)
      ;[0.15 0.15 0.15 0.5] destroys the old components
      (Components|DestroyComponent (Variables|Default|GetRenderComponent)))))

(event Collision|EventActorBeginOverlap
  (params (OtherActor :type Actor%20Object%20Reference)))

(event EventTick
  (params (DeltaSeconds :type Float%20%28single-precision%29)))

(fn ConstructionScript)