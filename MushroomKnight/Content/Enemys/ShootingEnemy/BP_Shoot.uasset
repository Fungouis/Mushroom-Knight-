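; Shooting enemy character that patrols by constantly walking forward at reduced input.
; When its Floor sensor ends an overlap or its Wall sensor begins one, it waits briefly, flips around, and spawns a bullet at Spawnshoot, destroying it a second later.
; Firing is therefore tied to patrol turns rather than player detection.
; Damage lowers SmallHealth, and at zero the enemy spawns a pickup and destroys itself.
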(event OnComponentEndOverlap(Floor)
  (params (OverlappedComponent :type Primitive%20Component%20Object%20Reference) (OtherActor :type Actor%20Object%20Reference) (OtherComp :type Primitive%20Component%20Object%20Reference) (OtherBodyIndex :type Integer))
  (bind _spawnshoot (Variables|Default|GetSpawnshoot))
  (Utilities|FlowControl|Delay 1.4)
  (CallFunction|TurnAround)
  (bind _returnvalue (Game|SpawnActorfromClass "/Game/Enemys/ShootingEnemy/BP_bullet.BP_bullet_C" (Transformation|GetWorldTransform _spawnshoot) "Undefined" "MultiplyWithRoot" 0 0))
  (Utilities|FlowControl|Delay 1.0)
  (Actor|DestroyActor _returnvalue)
  (Utilities|IsValid _spawnshoot))

(event OnComponentBeginOverlap(wall)
  (params (OverlappedComponent :type Primitive%20Component%20Object%20Reference) (OtherActor :type Actor%20Object%20Reference) (OtherComp :type Primitive%20Component%20Object%20Reference) (OtherBodyIndex :type Integer) (bFromSweep :type Boolean) (SweepResult :type Hit%20Result%20Structure%20%28by%20ref%29))
  (bind _spawnshoot (Variables|Default|GetSpawnshoot))
  (Utilities|FlowControl|Delay 1.4)
  (CallFunction|TurnAround)
  (bind _returnvalue (Game|SpawnActorfromClass "/Game/Enemys/ShootingEnemy/BP_bullet.BP_bullet_C" (Transformation|GetWorldTransform _spawnshoot) "Undefined" "MultiplyWithRoot" 0 0))
  (Utilities|FlowControl|Delay 1.0)
  (Actor|DestroyActor _returnvalue)
  (Utilities|IsValid _spawnshoot))

(event EventBeginPlay)

(event Collision|EventActorBeginOverlap
  (params (OtherActor :type Actor%20Object%20Reference)))

(event EventTick
  (params (DeltaSeconds :type Float%20%28single-precision%29))
  ;[0.15 0.15 0.15 0.5] Adds Movment
  (Pawn|Input|AddMovementInput (Transformation|GetActorForwardVector) 0.3 false))

(event Game|Damage|EventAnyDamage
  (params (Damage :type Float%20%28single-precision%29) (DamageType :type Damage%20Type%20Object%20Reference) (InstigatedBy :type Controller%20Object%20Reference) (DamageCauser :type Actor%20Object%20Reference))
  (Variables|Default|SetSmallHealth (- (Variables|Default|GetSmallHealth) Damage))
  (if (<= (Variables|Default|GetSmallHealth) 0.0)
    (Components|Activation|Deactivate (Variables|Character|GetCharacterMovement))
    (Game|SpawnActorfromClass "/Game/Pickups/BP_pickup.BP_pickup_C" (Transformation|GetActorTransform) "Undefined" "MultiplyWithRoot" 0 0)
    (Components|DestroyComponent (Variables|Collision|GetCapsuleComponent))
    (Actor|DestroyActor)))

(fn ConstructionScript)

(fn TurnAround
  ;[0.15 0.15 0.15 0.5] Flips there sprite around
  (Transformation|SetActorRotation (Math|Rotator|CombineRotators (Transformation|GetActorRotation) "0.000000,180.000000,0.000000")))