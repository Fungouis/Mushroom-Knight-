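; BP_SmallEnemy is a flipbook skeleton enemy that patrols by constantly walking forward.
; It turns around when its Floor trigger ends an overlap or its Wall trigger begins one.
; Its Damage trigger hurts BP_Charchter, pausing movement for the attack animation before turning back.
; Lethal damage plays the death flipbook, spawns BP_pickup and removes movement and collision components, leaving the actor in place.
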(event OnComponentEndOverlap(Floor)
  (params (OverlappedComponent :type Primitive%20Component%20Object%20Reference) (OtherActor :type Actor%20Object%20Reference) (OtherComp :type Primitive%20Component%20Object%20Reference) (OtherBodyIndex :type Integer))
  (CallFunction|TurnAround)
  (Utilities|FlowControl|Delay 0.5))

(event OnComponentBeginOverlap(wall)
  (params (OverlappedComponent :type Primitive%20Component%20Object%20Reference) (OtherActor :type Actor%20Object%20Reference) (OtherComp :type Primitive%20Component%20Object%20Reference) (OtherBodyIndex :type Integer) (bFromSweep :type Boolean) (SweepResult :type Hit%20Result%20Structure%20%28by%20ref%29))
  (CallFunction|TurnAround)
  (Utilities|FlowControl|Delay 0.5))

(event OnComponentBeginOverlap(Damage)
  (params (OverlappedComponent :type Primitive%20Component%20Object%20Reference) (OtherActor :type Actor%20Object%20Reference) (OtherComp :type Primitive%20Component%20Object%20Reference) (OtherBodyIndex :type Integer) (bFromSweep :type Boolean) (SweepResult :type Hit%20Result%20Structure%20%28by%20ref%29))
  (bind _asbp_charchter (Utilities|Casting|CastToBP_Charchter OtherActor))
  (Variables|Default|SetAttacking true)
  (Sprite|SetFlipbook (Variables|Default|GetSprite) "/Game/Enemys/Skeltonart/skelattack.skelattack")
  (Default|PlayerDamaged _asbp_charchter 1)
  (Utilities|FlowControl|Delay 0.7)
  (Variables|Default|SetAttacking false)
  (CallFunction|TurnAround)
  (Sprite|SetFlipbook (Variables|Default|GetSprite) "/Game/Enemys/Skeltonart/Skelwalk.Skelwalk")
  (Components|Timeline|SetLooping (Variables|Default|GetSprite) true))

(event EventBeginPlay)

(event Collision|EventActorBeginOverlap
  (params (OtherActor :type Actor%20Object%20Reference)))

(event EventTick
  (params (DeltaSeconds :type Float%20%28single-precision%29))
  ;[0.15 0.15 0.15 0.5] Adds Movment
  (if (not (Variables|Default|GetAttacking))
    (Pawn|Input|AddMovementInput (Transformation|GetActorForwardVector) 0.3 false)))

(event Game|Damage|EventAnyDamage
  (params (Damage :type Float%20%28single-precision%29) (DamageType :type Damage%20Type%20Object%20Reference) (InstigatedBy :type Controller%20Object%20Reference) (DamageCauser :type Actor%20Object%20Reference))
  (Variables|Default|SetSmallHealth (- (Variables|Default|GetSmallHealth) Damage))
  (if (<= (Variables|Default|GetSmallHealth) 0.0)
    (Sprite|SetFlipbook (Variables|Default|GetSprite) "/Game/Enemys/Skeltonart/Skellodeath.Skellodeath")
    (Components|Timeline|SetLooping (Variables|Default|GetSprite) false)
    (Components|Activation|Deactivate (Variables|Character|GetCharacterMovement))
    (Game|SpawnActorfromClass "/Game/Pickups/BP_pickup.BP_pickup_C" (Transformation|GetActorTransform) "Undefined" "MultiplyWithRoot" 0 0)
    (Components|DestroyComponent (Variables|Default|GetDamage))))

(fn ConstructionScript)

(fn TurnAround
  ;[0.15 0.15 0.15 0.5] Flips there sprite around
  (Transformation|SetActorRotation (Math|Rotator|CombineRotators (Transformation|GetActorRotation) "0.000000,180.000000,0.000000")))