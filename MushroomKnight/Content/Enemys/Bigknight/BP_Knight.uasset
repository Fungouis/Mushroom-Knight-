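; BP_Knight is a flipbook-animated patrolling enemy that damages BP_Charchter on contact.
; It walks forward unless attacking, turning around when the Floor sensor ends overlap or the Wall sensor begins one.
; The Damage overlap triggers a DoOnce-gated attack, then a turn and return to walking.
; Hits launch it away from the player; death plays a flipbook, disables movement and collision components, and spawns BP_pickup.
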(event OnComponentEndOverlap(Floor)
  (params (OverlappedComponent :type Primitive%20Component%20Object%20Reference) (OtherActor :type Actor%20Object%20Reference) (OtherComp :type Primitive%20Component%20Object%20Reference) (OtherBodyIndex :type Integer))
  (CallFunction|TurnAround)
  (Utilities|FlowControl|Delay 0.5))

(event OnComponentBeginOverlap(wall)
  (params (OverlappedComponent :type Primitive%20Component%20Object%20Reference) (OtherActor :type Actor%20Object%20Reference) (OtherComp :type Primitive%20Component%20Object%20Reference) (OtherBodyIndex :type Integer) (bFromSweep :type Boolean) (SweepResult :type Hit%20Result%20Structure%20%28by%20ref%29))
  (CallFunction|TurnAround)
  (Utilities|FlowControl|Delay 0.5))

(event OnComponentBeginOverlap(Damage)
  (params (OverlappedComponent :type Primitive%20Component%20Object%20Reference) (OtherActor :type Actor%20Object%20Reference) (OtherComp :type Primitive%20Component%20Object%20Reference) (OtherBodyIndex :type Integer) (bFromSweep :type Boolean) (SweepResult :type Hit%20Result%20Structure%20%28by%20ref%29))
  (bind _asbp_charchter (Utilities|Casting|CastToBP_Charchter OtherActor))
  (Utilities|FlowControl|DoOnce false :!label _label
    (:Completed
      (Variables|Default|SetAttacking true)
      (Sprite|SetFlipbook (Variables|Default|GetSprite) "/Game/Enemys/Bigknight/knightattack.knightattack")
      (Default|PlayerDamaged _asbp_charchter 1)
      (Utilities|FlowControl|Delay 0.7)
      (Variables|Default|SetAttacking false)
      (CallFunction|TurnAround)
      (Sprite|SetFlipbook (Variables|Default|GetSprite) "/Game/Enemys/Bigknight/knighwalk.knighwalk")
      (Components|Timeline|SetLooping (Variables|Default|GetSprite) true)
      (goto _label Reset))))

(event EventTick
  (params (DeltaSeconds :type Float%20%28single-precision%29))
  (if (not (Variables|Default|GetAttacking))
    (Pawn|Input|AddMovementInput (Transformation|GetActorForwardVector) 0.2 false)))

(event Game|Damage|EventAnyDamage
  (params (Damage :type Float%20%28single-precision%29) (DamageType :type Damage%20Type%20Object%20Reference) (InstigatedBy :type Controller%20Object%20Reference) (DamageCauser :type Actor%20Object%20Reference))
  (Variables|Default|SetSmallHealth (- (Variables|Default|GetSmallHealth) Damage))
  (if (<= (Variables|Default|GetSmallHealth) 0.0)
    (Audio|PlaySound2D "/Game/sounds/hurtenemy.hurtenemy" 1.0 1.0 0.0 0 0)
    (Sprite|SetFlipbook (Variables|Default|GetSprite) "/Game/Enemys/Bigknight/knightdeath.knightdeath")
    (Components|Timeline|SetLooping (Variables|Default|GetSprite) false)
    (Components|Activation|Deactivate (Variables|Character|GetCharacterMovement))
    (Game|SpawnActorfromClass "/Game/Pickups/BP_pickup.BP_pickup_C" (Transformation|GetActorTransform) "Undefined" "MultiplyWithRoot" 0 0)
    (Components|DestroyComponent (Variables|Default|GetDamage))
    (else
      (Audio|PlaySound2D "/Game/sounds/hurtenemy.hurtenemy" 1.0 1.0 0.0 0 0)
      (Character|LaunchCharacter (Math|Vector|MakeVector (.x (* (Math|Vector|GetUnitDirection(Vector) (Transformation|GetActorLocation (Game|GetPlayerCharacter 0)) (Transformation|GetActorLocation)) 5e+01)) 0.0 1.8e+02) true true))))

(fn ConstructionScript)

(fn TurnAround
  (Transformation|SetActorRotation (Math|Rotator|CombineRotators (Transformation|GetActorRotation) "0.000000,180.000000,0.000000")))