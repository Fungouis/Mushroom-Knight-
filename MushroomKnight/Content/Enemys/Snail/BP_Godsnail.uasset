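; BP_Godsnail is a flipbook-sprite snail enemy that patrols by constantly walking forward at reduced input.
; It turns around when its Floor probe loses overlap, its Wall probe hits, or its Damage volume touches the player, who takes damage.
; Taking damage launches it along a fixed world direction; at zero health it plays a death flipbook, stops moving, spawns a pickup and destroys its capsule, Wall and Damage components.
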(event OnComponentEndOverlap(Floor)
  (params (OverlappedComponent :type Primitive%20Component%20Object%20Reference) (OtherActor :type Actor%20Object%20Reference) (OtherComp :type Primitive%20Component%20Object%20Reference) (OtherBodyIndex :type Integer))
  (CallFunction|TurnAround))

(event OnComponentBeginOverlap(wall)
  (params (OverlappedComponent :type Primitive%20Component%20Object%20Reference) (OtherActor :type Actor%20Object%20Reference) (OtherComp :type Primitive%20Component%20Object%20Reference) (OtherBodyIndex :type Integer) (bFromSweep :type Boolean) (SweepResult :type Hit%20Result%20Structure%20%28by%20ref%29))
  (CallFunction|TurnAround))

(event OnComponentBeginOverlap(Damage)
  (params (OverlappedComponent :type Primitive%20Component%20Object%20Reference) (OtherActor :type Actor%20Object%20Reference) (OtherComp :type Primitive%20Component%20Object%20Reference) (OtherBodyIndex :type Integer) (bFromSweep :type Boolean) (SweepResult :type Hit%20Result%20Structure%20%28by%20ref%29))
  (bind _asbp_charchter (Utilities|Casting|CastToBP_Charchter OtherActor))
  (CallFunction|TurnAround)
  (Default|PlayerDamaged _asbp_charchter 1))

(event EventBeginPlay)

(event Collision|EventActorBeginOverlap
  (params (OtherActor :type Actor%20Object%20Reference)))

(event EventTick
  (params (DeltaSeconds :type Float%20%28single-precision%29))
  (Pawn|Input|AddMovementInput (Transformation|GetActorForwardVector) 0.3 false))

(event Game|Damage|EventAnyDamage
  (params (Damage :type Float%20%28single-precision%29) (DamageType :type Damage%20Type%20Object%20Reference) (InstigatedBy :type Controller%20Object%20Reference) (DamageCauser :type Actor%20Object%20Reference))
  (Variables|Default|SetSmallHealth (- (Variables|Default|GetSmallHealth) Damage))
  (if (<= (Variables|Default|GetSmallHealth) 0.0)
    (Sprite|SetFlipbook (Variables|Default|GetSprite) "/Game/Enemys/Snail/Dead-Snail.Dead-Snail")
    (Components|Timeline|SetLooping (Variables|Default|GetSprite) false)
    (Components|Activation|Deactivate (Variables|Character|GetCharacterMovement))
    (Game|SpawnActorfromClass "/Game/Pickups/BP_pickup.BP_pickup_C" (Transformation|GetActorTransform) "Undefined" "MultiplyWithRoot" 0 0)
    (Components|DestroyComponent (Variables|Default|GetDamage))
    (else
      (Character|LaunchCharacter "100.000000,0.000000,100.000000" true true))))

(fn ConstructionScript)

(fn TurnAround
  (Transformation|SetActorRotation (Math|Rotator|CombineRotators (Transformation|GetActorRotation) "0.000000,180.000000,0.000000")))