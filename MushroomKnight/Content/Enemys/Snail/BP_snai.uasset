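; Snail enemy character with a flipbook sprite that patrols by constantly moving along its forward vector.
; It flips around when its Floor probe loses overlap or its Wall probe gains one.
; Touching BP_Charchter via the Damage component also turns it and deals damage, gated by a short cooldown.
; Hits knock it away from the player; at zero health it plays a death flipbook, shuts down movement and collision components, and spawns BP_pickup.
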(event OnComponentEndOverlap(Floor)
  (params (OverlappedComponent :type Primitive%20Component%20Object%20Reference) (OtherActor :type Actor%20Object%20Reference) (OtherComp :type Primitive%20Component%20Object%20Reference) (OtherBodyIndex :type Integer))
  (Variables|Default|SetCan%20Turn true)
  (Utilities|FlowControl|DoOnce false :!label _label
    (:Completed
      (CallFunction|TurnAround)
      (goto _label Reset))))

(event OnComponentBeginOverlap(wall)
  (params (OverlappedComponent :type Primitive%20Component%20Object%20Reference) (OtherActor :type Actor%20Object%20Reference) (OtherComp :type Primitive%20Component%20Object%20Reference) (OtherBodyIndex :type Integer) (bFromSweep :type Boolean) (SweepResult :type Hit%20Result%20Structure%20%28by%20ref%29))
  (Variables|Default|SetCan%20Turn true)
  (Utilities|FlowControl|DoOnce false :!label _label
    (:Completed
      (CallFunction|TurnAround)
      (goto _label Reset))))

(event OnComponentBeginOverlap(Damage)
  (params (OverlappedComponent :type Primitive%20Component%20Object%20Reference) (OtherActor :type Actor%20Object%20Reference) (OtherComp :type Primitive%20Component%20Object%20Reference) (OtherBodyIndex :type Integer) (bFromSweep :type Boolean) (SweepResult :type Hit%20Result%20Structure%20%28by%20ref%29))
  (bind _asbp_charchter (Utilities|Casting|CastToBP_Charchter OtherActor))
  (Utilities|FlowControl|DoOnce false :!label _label
    (:Completed
      (CallFunction|TurnAround)
      (Default|PlayerDamaged _asbp_charchter 1)
      (Utilities|FlowControl|Delay 0.7)
      (goto _label Reset))))

(event EventBeginPlay)

(event Collision|EventActorBeginOverlap
  (params (OtherActor :type Actor%20Object%20Reference)))

(event EventTick
  (params (DeltaSeconds :type Float%20%28single-precision%29))
  (Pawn|Input|AddMovementInput (Transformation|GetActorForwardVector) (Variables|Default|GetSpeed) false))

(event Game|Damage|EventAnyDamage
  (params (Damage :type Float%20%28single-precision%29) (DamageType :type Damage%20Type%20Object%20Reference) (InstigatedBy :type Controller%20Object%20Reference) (DamageCauser :type Actor%20Object%20Reference))
  (Variables|Default|SetSmallHealth (- (Variables|Default|GetSmallHealth) Damage))
  (if (<= (Variables|Default|GetSmallHealth) 0.0)
    (Audio|PlaySound2D "/Game/sounds/hurtenemy.hurtenemy" 1.0 1.0 0.0 0 0)
    (Sprite|SetFlipbook (Variables|Default|GetSprite) "/Game/Enemys/Snail/Dead-Snail.Dead-Snail")
    (Components|Timeline|SetLooping (Variables|Default|GetSprite) false)
    (Components|Activation|Deactivate (Variables|Character|GetCharacterMovement))
    (Game|SpawnActorfromClass "/Game/Pickups/BP_pickup.BP_pickup_C" (Transformation|GetActorTransform) "Undefined" "MultiplyWithRoot" 0 0)
    (Components|Activation|Deactivate (Variables|Default|GetDamage))
    (else
      (Audio|PlaySound2D "/Game/sounds/hurtenemy.hurtenemy" 1.0 1.0 0.0 0 0)
      (Character|LaunchCharacter (Math|Vector|MakeVector (.x (* (Math|Vector|GetUnitDirection(Vector) (Transformation|GetActorLocation (Game|GetPlayerCharacter 0)) (Transformation|GetActorLocation)) 1e+02)) 0.0 1.8e+02) true true))))

(fn ConstructionScript)

(fn TurnAround
  (Transformation|SetActorRotation (Math|Rotator|CombineRotators (Transformation|GetActorRotation) "0.000000,180.000000,0.000000")))