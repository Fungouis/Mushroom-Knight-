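; BP_Shoot is a shooting bee enemy character that patrols by constantly moving forward.
; Its Floor end-overlap and Wall begin-overlap events share one delayed path that turns it around, fires a BP_bullet from Spawnshoot and destroys the bullet shortly after.
; Damage reduces SmallHealth and knocks it up and away from the player; at zero it drops a BP_pickup, spawns a poof effect and destroys itself.
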(event OnComponentEndOverlap(Floor)
  (params (OverlappedComponent :type Primitive%20Component%20Object%20Reference) (OtherActor :type Actor%20Object%20Reference) (OtherComp :type Primitive%20Component%20Object%20Reference) (OtherBodyIndex :type Integer))
  ;[0.15 0.15 0.15 0.5] Checks for floor/wall
  ;[0.15 0.15 0.15 0.5] Delay to when turn
  (Utilities|FlowControl|Delay (Variables|movement|GetTime%20to%20turn))
  ;[0.15 0.15 0.15 0.5] Turns them around
  (CallFunction|TurnAround)
  ;[0.15 0.15 0.15 0.5] Spawns there bullet
  (bind _returnvalue (Game|SpawnActorfromClass "/Game/Enemys/beee/BP_bullet.BP_bullet_C" (Transformation|GetWorldTransform (Variables|Default|GetSpawnshoot)) "Undefined" "MultiplyWithRoot" 0 0))
  ;[0.15 0.15 0.15 0.5] Checks if vaild then destroys it if is
  (Utilities|FlowControl|Delay 1.0)
  (Utilities|IsValid _returnvalue
    (:Is%20Valid
      (Actor|DestroyActor _returnvalue))))

(event OnComponentBeginOverlap(wall)
  (params (OverlappedComponent :type Primitive%20Component%20Object%20Reference) (OtherActor :type Actor%20Object%20Reference) (OtherComp :type Primitive%20Component%20Object%20Reference) (OtherBodyIndex :type Integer) (bFromSweep :type Boolean) (SweepResult :type Hit%20Result%20Structure%20%28by%20ref%29))
  ;[0.15 0.15 0.15 0.5] Checks for floor/wall
  ;[0.15 0.15 0.15 0.5] Delay to when turn
  (Utilities|FlowControl|Delay (Variables|movement|GetTime%20to%20turn))
  ;[0.15 0.15 0.15 0.5] Turns them around
  (CallFunction|TurnAround)
  ;[0.15 0.15 0.15 0.5] Spawns there bullet
  (bind _returnvalue (Game|SpawnActorfromClass "/Game/Enemys/beee/BP_bullet.BP_bullet_C" (Transformation|GetWorldTransform (Variables|Default|GetSpawnshoot)) "Undefined" "MultiplyWithRoot" 0 0))
  ;[0.15 0.15 0.15 0.5] Checks if vaild then destroys it if is
  (Utilities|FlowControl|Delay 1.0)
  (Utilities|IsValid _returnvalue
    (:Is%20Valid
      (Actor|DestroyActor _returnvalue))))

(event EventTick
  (params (DeltaSeconds :type Float%20%28single-precision%29))
  ;[0.15 0.15 0.15 0.5] Adds Movment
  (Pawn|Input|AddMovementInput (Transformation|GetActorForwardVector) 0.3 false))

(event Game|Damage|EventAnyDamage
  (params (Damage :type Float%20%28single-precision%29) (DamageType :type Damage%20Type%20Object%20Reference) (InstigatedBy :type Controller%20Object%20Reference) (DamageCauser :type Actor%20Object%20Reference))
  ;[0.15 0.15 0.15 0.5] Checks of there  healt has taken Damage
  (Variables|health|SetSmallHealth (- (Variables|health|GetSmallHealth) Damage))
  ;[0.15 0.15 0.15 0.5] If  = 0 moves to dead
  (if (<= (Variables|health|GetSmallHealth) 0.0)
    ;[0.15 0.15 0.15 0.5] Hurt sound
    (Audio|PlaySound2D "/Game/sounds/hurtenemy.hurtenemy" 1.0 1.0 0.0 0 0)
    ;[0.15 0.15 0.15 0.5] Stops movment
    (Components|Activation|Deactivate (Variables|Character|GetCharacterMovement))
    ;[0.15 0.15 0.15 0.5] Spawns points
    (Game|SpawnActorfromClass "/Game/Pickups/BP_pickup.BP_pickup_C" (Transformation|GetActorTransform) "Undefined" "MultiplyWithRoot" 0 0)
    (Niagara|SpawnSystematLocation "/Game/FX/NS_beepoof.NS_beepoof" (Transformation|GetWorldLocation (Variables|Default|GetSprite)))
    ;[0.15 0.15 0.15 0.5] Disables there componets
    (Components|DestroyComponent (Variables|Collision|GetCapsuleComponent))
    ;[0.15 0.15 0.15 0.5] Destroys them
    (Actor|DestroyActor)
    (else
      (Audio|PlaySound2D "/Game/sounds/hurtenemy.hurtenemy" 1.0 1.0 0.0 0 0)
      ;[0.15 0.15 0.15 0.5] Launch them away from the player
      (Character|LaunchCharacter (Math|Vector|MakeVector (.x (* (Math|Vector|GetUnitDirection(Vector) (Transformation|GetActorLocation (Game|GetPlayerCharacter 0)) (Transformation|GetActorLocation)) 5e+01)) 0.0 1.8e+02) true true))))

(fn ConstructionScript)

(fn TurnAround
  ;[0.15 0.15 0.15 0.5] Flips there sprite around
  (Transformation|SetActorRotation (Math|Rotator|CombineRotators (Transformation|GetActorRotation) "0.000000,180.000000,0.000000")))